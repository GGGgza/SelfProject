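; BP_Enemies_Base is an enemy base Blueprint that provides a single melee attack.
; Attack_01 plays a two-handed attack montage on the Mesh, then calls the CallOnAttackEnd dispatcher whether the montage completes or is interrupted.
; Tick, BeginPlay and the construction script are empty.
; An unconnected debug print holds a dot-product test for whether the player is in front of the enemy.
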(event `self.ReceiveTick`
  (params (DeltaSeconds :type "Float (single-precision)")))

(event `Attack_01`
  (`|PlayMontage` (`self.Mesh`) "/Game/Enemies/Anim/2H_Attack_C_MontageRoot.2H_Attack_C_MontageRoot"
    (:`OnCompleted`
      _)
    (:`OnInterrupted`
      _))
  (`self.Call On Attack End`))

(event `self.ReceiveBeginPlay`)

(fn `UserConstructionScript`)